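; BP_DungeonGrid is an actor that builds a randomized dungeon tile grid on BeginPlay.
; It fills a Tiles array of room info structs, picking one of two tile types by RoomPercent chance, a placeholder for a real algorithm.
; Debug mode, always on at BeginPlay, draws each tile as a box colored by type.
; Row index divides by GridHeight rather than GridWidth, so coordinates assume a square grid.
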(event EventBeginPlay
  (CallFunction|InitializeGrid true))

(event Collision|EventActorBeginOverlap
  (params (OtherActor :type Actor%20Object%20Reference)))

(event EventTick
  (params (DeltaSeconds :type Float%20%28single-precision%29)))

(fn ConstructionScript)

(fn InitializeGrid
  (params (DebugMode :type Boolean))
  (|MakeTilesArray
    (:Completed
      (if DebugMode
        (CallFunction|DrawTileDebugBox 6e+02 15.0)
        (else
          (return))))))

(fn DrawTileDebugBox
  (params (DebugDrawDuration :type Float%20%28double-precision%29) (BoxThickness :type Float%20%28single-precision%29))
  (for _array_element (Variables|Default|GetTiles)
    (Rendering|Debug|DrawDebugBox _array_element DebugDrawDuration BoxThickness))
  (return))

(fn GetTileType
  ;[0.15 0.15 0.15 0.5] Make a real algorithm
  (if (< (Math|Random|RandomInteger 100) (Variables|TileTypePercentages|GetRoomPercent))
    (LocalVariables|SetTileType 1)
    (else
      (LocalVariables|SetTileType 0)))
  (return (Utilities|Select :Index (LocalVariables|GetTileType) :Option%200 "NewEnumerator0" :Option%201 "NewEnumerator1" :Option%202 "NewEnumerator2")))